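; BP_Enemy is a flipbook-animated Bandit enemy that takes damage, dies and awards EXP to the player.
; On spawn it caches the player and HP widget, then yaws its capsule from the player's spring arm.
; Damage updates health and the widget, which a sphere overlap shows or hides.
; Tick picks idle or run by velocity, overriding hit and death flipbooks, and flips the sprite by Y velocity.
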(event `self.ReceiveAnyDamage`
  (params (Damage :type "Float (single-precision)") (DamageType :type "DamageType Object Reference") (InstigatedBy :type "Controller Object Reference") (DamageCauser :type "Actor Object Reference"))
  (`PaperFlipbookComponent.SetFlipbook` (`self.Sprite`) "/Game/Assets/Animations/Enemies/Into_The_Journey/Bandit_F/Bandit_-_F_Hit.Bandit_-_F_Hit")
  (bind _output_get (set `self.Health` (`KismetMathLibrary.FClamp` (- (`self.Health`) Damage) 0.0 100.0)))
  (set `/Game/Blueprints/Enemy/BP_Enemy_HP.EnemyHealth` _output_get (`self.HP_REF`))
  (`KismetSystemLibrary.Delay` 0.2)
  (if (== _output_get 0.0)
    (`PaperFlipbookComponent.SetFlipbook` (`self.Sprite`) "/Game/Assets/Animations/Enemies/Into_The_Journey/Bandit_F/Bandit_-_F_Death.Bandit_-_F_Death")
    (`KismetSystemLibrary.Delay` 0.5)
    (`|ExecutionSequence`
      (:`then_0`
        (`self.K2_DestroyActor`))
      (:`then_1`
        (`/Game/Assets/Blueprints/BP_Character.Add EXP` (`self.CHAR_REF`) 5)))))

(event `self.Sphere.OnComponentBeginOverlap`
  (params (OverlappedComponent :type "PrimitiveComponent Object Reference") (OtherActor :type "Actor Object Reference") (OtherComp :type "PrimitiveComponent Object Reference") (OtherBodyIndex :type Integer) (bFromSweep :type Boolean) (SweepResult :type "HitResult Structure (by ref)"))
  (cast `/Game/Assets/Blueprints/BP_Character` OtherActor)
  (`SceneComponent.SetVisibility` (`self.HP_Widget`) true false))

(event `self.Sphere.OnComponentEndOverlap`
  (params (OverlappedComponent :type "PrimitiveComponent Object Reference") (OtherActor :type "Actor Object Reference") (OtherComp :type "PrimitiveComponent Object Reference") (OtherBodyIndex :type Integer))
  (cast `/Game/Assets/Blueprints/BP_Character` OtherActor)
  (`SceneComponent.SetVisibility` (`self.HP_Widget`) false false))

(event `self.ReceiveBeginPlay`
  (bind (_returnvalue_roll _returnvalue_pitch _returnvalue_yaw) (`KismetMathLibrary.BreakRotator` (`SceneComponent.K2_GetComponentRotation` (`self.GetComponentByClass` (`GameplayStatics.GetPlayerPawn` 0) "/Script/Engine.SpringArmComponent"))))
  ;[1 1 1] Fix World Rotation when Spawned
  (`|ExecutionSequence`
    (:`then_0`
      (bind _asbp_character (cast `/Game/Assets/Blueprints/BP_Character` (`GameplayStatics.GetPlayerCharacter` 0)))
      (set `self.CHAR_REF` _asbp_character)
      (bind _asbp_enemy_hp (cast `/Game/Blueprints/Enemy/BP_Enemy_HP` (`WidgetComponent.GetUserWidgetObject` (`self.HP_Widget`))))
      (set `self.HP_REF` _asbp_enemy_hp))
    (:`then_1`
      (`SceneComponent.K2_SetWorldRotation` (`self.CapsuleComponent`) (`KismetMathLibrary.MakeRotator` 0.0 0.0 (- _returnvalue_yaw 90.0)) false false))))

(event `self.ReceiveTick`
  (params (DeltaSeconds :type "Float (single-precision)"))
  ;[1 1 1] Animation
  (`self.Update Animation`)
  (`self.UpdateControlRotation`))

(event `Update Animation`
  ;[1 1 1] Animation
  (`PaperFlipbookComponent.SetFlipbook` (`self.Sprite`) (select `bool` (> (`KismetMathLibrary.VSize` (`MovementComponent.Velocity` (`self.CharacterMovement`))) 0.0) :`false` "/Game/Assets/Animations/Enemies/Into_The_Journey/Bandit_F/Bandit_-_F_Idle.Bandit_-_F_Idle" :`true` "/Game/Assets/Animations/Enemies/Into_The_Journey/Bandit_F/Bandit_-_F_Run.Bandit_-_F_Run" :!type "PaperFlipbook Object Reference")))

(event `UpdateControlRotation`
  (bind _sprite (`self.Sprite`))
  ;[1 1 1] Sprite Flip
  (`/Engine/EditorBlueprintResources/StandardMacros.IsValid` (`self.GetController`)
    (:`Is Valid`
      (`/Engine/EditorBlueprintResources/StandardMacros.CompareFloat` (`.Y` (`KismetMathLibrary.BreakVector3f` (`MovementComponent.Velocity` (`self.CharacterMovement`))))
        (:`>`
          (`SceneComponent.K2_SetRelativeRotation` _sprite (`KismetMathLibrary.MakeRotator` 0.0) false false))
        (:`<`
          (`SceneComponent.K2_SetRelativeRotation` _sprite (`KismetMathLibrary.MakeRotator` 0.0 0.0 180.0) false false))))))

(fn `UserConstructionScript`)