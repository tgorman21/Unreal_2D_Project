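; BP_Enemy is a Paper2D enemy that issues one AI Move To at BeginPlay, targeting player controller 0 rather than its pawn.
; Each Tick switches the sprite between Apprentice walk and idle flipbooks based on whether it is moving.
; It also yaws the sprite to face the sign of Y velocity while a controller is valid.
; A debug print and a player distance check are left unconnected.
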(event `self.ReceiveBeginPlay`
  (`|AIMoveTo` self (0.0 0.0 0.0) (`GameplayStatics.GetPlayerController` 0)))

(event `self.ReceiveTick`
  (params (DeltaSeconds :type "Float (single-precision)"))
  ;[1 1 1] Animation
  (`self.Update Animation`)
  (`self.UpdateControlRotation`))

(event `Update Animation`
  ;[1 1 1] Animation
  (`PaperFlipbookComponent.SetFlipbook` (`self.Sprite`) (select `bool` (> (`KismetMathLibrary.VSize` (`MovementComponent.Velocity` (`self.CharacterMovement`))) 0.0) :`false` "/Game/FUNTASY_World/Characters/Magician/Apprentice/FlipBoooks/Apprentice_Idle.Apprentice_Idle" :`true` "/Game/FUNTASY_World/Characters/Magician/Apprentice/FlipBoooks/Apprentice_Jump_Walk.Apprentice_Jump_Walk" :!type "PaperFlipbook Object Reference")))

(event `UpdateControlRotation`
  (bind _sprite (`self.Sprite`))
  ;[1 1 1] Sprite Flip
  (`/Engine/EditorBlueprintResources/StandardMacros.IsValid` (`self.GetController`)
    (:`Is Valid`
      (`/Engine/EditorBlueprintResources/StandardMacros.CompareFloat` (`.Y` (`KismetMathLibrary.BreakVector3f` (`MovementComponent.Velocity` (`self.CharacterMovement`))))
        (:`>`
          (`SceneComponent.K2_SetRelativeRotation` _sprite (`KismetMathLibrary.MakeRotator` 0.0) false false))
        (:`<`
          (`SceneComponent.K2_SetRelativeRotation` _sprite (`KismetMathLibrary.MakeRotator` 0.0 0.0 180.0) false false))))))

(fn `UserConstructionScript`)