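; Player character for a flipbook-sprite Apprentice, with movement, sprinting, three spawned attacks, health, mana, stamina and EXP leveling.
; Input and damage events set state flags that Tick turns into animations, alongside resource regeneration and velocity-based sprite flipping.
; Stat functions push values to BP_HUD, which also receives the death notice.
; Overlapping tagged enemies moves the spring arm to a higher, farther view via a timeline, reversed once none remain.
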(event `self.ReceiveTick`
  (params (DeltaSeconds :type "Float (single-precision)"))
  ;[1 1 1] Event Tick
  (if (`self.Attacking1`)
    (`self.Atk1`)
    (elif (`self.Attacking2`)
      (`self.Atk2`)
      (elif (`self.Attacking3`)
        (`self.Atk3`)
        (else
          (`self.Update Animation`)))))
  (`self.UpdateControlRotation`)
  (`self.UpdateSpringArm`)
  ;;[1 1 1] Mana Recharge
  (`self.UpdateMana` (+ (`self.mana`) 1.0))
  ;;[1 1 1] Sprint Recharge
  (if (not (`self.sprinting`))
    (`self.UpdateStamina` (+ (`self.stamina`) 0.3))))

(event `InputAction|Attack1`
  (params (Key :type "Key Structure"))
  (bind _mana (`self.mana`))
  ;[1 1 1] Attack 1 (projectile)
  (:`Pressed`
    (if (and (`self.canMove`) (not (`self.isDead`)))
      (if (> _mana 10.0)
        (set `self.Attacking1` true)
        (`KismetSystemLibrary.Delay` 0.2)
        (`|SpawnActorFromClass` "/Game/Assets/Animations/Characters/Mage/Apprentice/Attack_Items/Ranged_Attack1.Ranged_Attack1_C" (`SceneComponent.K2_GetComponentToWorld` (`self.Arrow1`)) "Undefined" "OverrideRootScale" null null)
        (`self.UpdateMana` (- _mana 10.0))
        (`KismetSystemLibrary.Delay` 0.3)
        (set `self.Attacking1` false)))))

(event `self.ReceiveAnyDamage`
  (params (Damage :type "Float (single-precision)") (DamageType :type "DamageType Object Reference") (InstigatedBy :type "Controller Object Reference") (DamageCauser :type "Actor Object Reference"))
  ;[1 1 1] Health
  (bind _output_get (set `self.Health` (`KismetMathLibrary.FClamp` (- (`self.health`) Damage) 0.0 100.0)))
  (if (== _output_get 0.0)
    (set `self.isDead` true)
    (else
      (set `self.isDamaged` true)
      (`self.UpdateHealth` _output_get))))

(event `Update Animation`
  (bind _returnvalue (`GameplayStatics.GetPlayerController` 0))
  (bind _sprite (`self.Sprite`))
  (bind _sprite_2 (`self.Sprite`))
  ;[1 1 1] Animation
  (if (`self.isDead`)
    (if (not (`self.deathScreenOn`))
      (`PaperFlipbookComponent.SetLooping` _sprite false)
      (`PaperFlipbookComponent.SetFlipbook` _sprite "/Game/Assets/Animations/Characters/Mage/Apprentice/Apprentice_Death.Apprentice_Death")
      (set `PlayerController.bShowMouseCursor` false _returnvalue)
      (bind _asbp_hud (cast `/Game/Blueprints/BP_HUD` (`PlayerController.GetHUD` _returnvalue)))
      (`/Game/Blueprints/BP_HUD.OnPlayerDeath` _asbp_hud)
      (set `self.deathScreenOn` true))
    (elif (`self.isDamaged`)
      (`PaperFlipbookComponent.SetFlipbook` _sprite_2 "/Game/Assets/Animations/Characters/Mage/Apprentice/Apprentice_Hit.Apprentice_Hit")
      (`KismetSystemLibrary.Delay` (`PaperFlipbookComponent.GetFlipbookLength` _sprite_2))
      (set `self.isDamaged` false)
      (else
        (`PaperFlipbookComponent.SetFlipbook` _sprite_2 (select `bool` (> (`KismetMathLibrary.VSize` (`MovementComponent.Velocity` (`self.CharacterMovement`))) 0.0) :`false` "/Game/Assets/Animations/Characters/Mage/Apprentice/Apprentice_Idle.Apprentice_Idle" :`true` "/Game/Assets/Animations/Characters/Mage/Apprentice/Apprentice_Run.Apprentice_Run" :!type "PaperFlipbook Object Reference"))))))

(event `Key|Four`
  (params (Key :type "Key Structure"))
  (:`Pressed`
    (`self.Add EXP` 5)))

(event `InputAxis|MoveRight`
  (params (AxisValue :type "Float (single-precision)"))
  (bind _stamina (`self.stamina`))
  ;[1 1 1] Movement
  (if (and (`self.canMove`) (not (`self.isDead`)))
    (`self.AddMovementInput` (`KismetMathLibrary.TransformDirection` (`self.GetTransform`) (0.0 1.0 0.0)) AxisValue)
    ;[1 1 1] Stamina
    (if (and (`NavMovementComponent.IsMovingOnGround` (`self.CharacterMovement`)) (`self.sprinting`)) :!label _label
      (`self.UpdateStamina` (- _stamina 0.1))
      (if (<= _stamina 0.0)
        ;[1 1 1] Sprint
        (set `CharacterMovementComponent.MaxWalkSpeed` 500.0 (`self.CharacterMovement`) :!label _label_2)
        (set `self.sprinting` false)))))

(event `Atk1`
  ;[1 1 1] Animation
  (`PaperFlipbookComponent.SetFlipbook` (`self.Sprite`) "/Game/Assets/Animations/Characters/Mage/Apprentice/Apprentice_Attack1.Apprentice_Attack1")
  (`MovementComponent.StopMovementImmediately` (`self.CharacterMovement`) :!label _label_3))

(event `Atk2`
  ;[1 1 1] Animation
  (`PaperFlipbookComponent.SetFlipbook` (`self.Sprite`) "/Game/Assets/Animations/Characters/Mage/Apprentice/Apprentice_Attack2.Apprentice_Attack2")
  (goto _label_3))

(event `InputAction|Attack2`
  (params (Key :type "Key Structure"))
  ;[1 1 1] Animation
  (:`Pressed`
    (if (and (`self.canMove`) (not (`self.isDead`)))
      (set `self.Attacking2` true)
      (`KismetSystemLibrary.Delay` 0.2)
      (bind _returnvalue (`|SpawnActorFromClass` "/Game/Assets/Animations/Characters/Mage/Apprentice/Attack_Items/Ranged_Attack2.Ranged_Attack2_C" (`SceneComponent.K2_GetComponentToWorld` (`self.Arrow1`)) "Undefined" "OverrideRootScale" null null))
      (`KismetSystemLibrary.Delay` 0.3)
      (`self.K2_DestroyActor` _returnvalue)
      (set `self.Attacking2` false))))

(event `InputAxis|MoveUp`
  (params (AxisValue :type "Float (single-precision)"))
  ;[1 1 1] Movement
  (if (and (`self.canMove`) (not (`self.isDead`)))
    (`self.AddMovementInput` (`KismetMathLibrary.TransformDirection` (`self.GetTransform`) (-1.0 0.0 0.0)) AxisValue)
    (goto _label)))

(event `Atk3`
  ;[1 1 1] Animation
  (`PaperFlipbookComponent.SetFlipbook` (`self.Sprite`) "/Game/Assets/Animations/Characters/Mage/Apprentice/Apprentice_Attack3.Apprentice_Attack3")
  (goto _label_3))

(event `InputAction|Sprint`
  (params (Key :type "Key Structure"))
  ;[1 1 1] Sprint
  (:`Pressed`
    (if (not (<= (`self.stamina`) 0.0))
      (set `CharacterMovementComponent.MaxWalkSpeed` 1000.0 (`self.CharacterMovement`))
      (set `self.sprinting` true)))
  (:`Released`
    (goto _label_2)))

(event `InputAction|Attack3`
  (params (Key :type "Key Structure"))
  ;[1 1 1] Animation
  (:`Pressed`
    (if (and (`self.canMove`) (not (`self.isDead`)))
      (set `self.Attacking3` true)
      (`KismetSystemLibrary.Delay` 0.2)
      (bind _returnvalue (`|SpawnActorFromClass` "/Game/Assets/Animations/Characters/Mage/Apprentice/Attack_Items/Ranged_Attack3.Ranged_Attack3_C" (`SceneComponent.K2_GetComponentToWorld` (`self.Arrow1`)) "Undefined" "OverrideRootScale" null null))
      (`KismetSystemLibrary.Delay` 0.3)
      (`self.K2_DestroyActor` _returnvalue)
      (set `self.Attacking3` false))))

(event `UpdateControlRotation`
  (bind _returnvalue (`self.GetController`))
  (bind _sprite (`self.Sprite`))
  (bind (_returnvalue_x _returnvalue_y) (`KismetMathLibrary.BreakVector` (`KismetMathLibrary.LessLess_VectorRotator` (`MovementComponent.Velocity` (`self.CharacterMovement`)) (`self.K2_GetActorRotation` _returnvalue))))
  ;[1 1 1] Sprite Flip
  (`/Engine/EditorBlueprintResources/StandardMacros.IsValid` _returnvalue
    (:`Is Valid`
      (`/Engine/EditorBlueprintResources/StandardMacros.CompareFloat` _returnvalue_y
        (:`>`
          (`SceneComponent.K2_SetRelativeRotation` _sprite (`KismetMathLibrary.MakeRotator` 0.0 0.0 90.0) false false))
        (:`<`
          (`SceneComponent.K2_SetRelativeRotation` _sprite (`KismetMathLibrary.MakeRotator` 0.0 0.0 -90.0) false false))))))

(event `self.EnemyTrigger.OnComponentBeginOverlap`
  (params (OverlappedComponent :type "PrimitiveComponent Object Reference") (OtherActor :type "Actor Object Reference") (OtherComp :type "PrimitiveComponent Object Reference") (OtherBodyIndex :type Integer) (bFromSweep :type Boolean) (SweepResult :type "HitResult Structure (by ref)"))
  ;[1 1 1] Move Spring Arm
  (if (`self.ActorHasTag` OtherActor "Enemy")
    (`BlueprintSetLibrary.Set_Add` (`self.overlappedEnemies`) OtherActor)
    (set `self.springArmPitch` -35.0)
    (set `self.springArmLength` 1500.0)))

(event `self.ReceiveBeginPlay`
  ;[1 1 1] Move Spring Arm
  (set `self.springArmPitch` -20.0 :!label _label_4)
  (set `self.springArmLength` 1200.0))

(event `self.EnemyTrigger.OnComponentEndOverlap`
  (params (OverlappedComponent :type "PrimitiveComponent Object Reference") (OtherActor :type "Actor Object Reference") (OtherComp :type "PrimitiveComponent Object Reference") (OtherBodyIndex :type Integer))
  (bind _overlappedenemies (`self.overlappedEnemies`))
  ;[1 1 1] Move Spring Arm
  (bind _returnvalue (`BlueprintSetLibrary.Set_Remove` _overlappedenemies OtherActor))
  (if _returnvalue
    (if (`BlueprintSetLibrary.Set_IsEmpty` _overlappedenemies)
      (goto _label_4))))

(event `UpdateSpringArm`
  (bind _springarm (`self.SpringArm`))
  (bind _springarmlength (`self.springArmLength`))
  (bind _springarm_2 (`self.SpringArm`))
  (bind (_relativerotation_roll _relativerotation_pitch) (`KismetMathLibrary.BreakRotator` (`SceneComponent.RelativeRotation` _springarm)))
  (bind _targetarmlength (`SpringArmComponent.TargetArmLength` _springarm))
  (bind (_relativerotation_roll_2 _relativerotation_pitch_2 _relativerotation_yaw) (`KismetMathLibrary.BreakRotator` (`SceneComponent.RelativeRotation` _springarm_2)))
  ;[1 1 1] Move Spring Arm
  (if (or (!= _targetarmlength _springarmlength) (!= (`self.springArmPitch`) _relativerotation_pitch))
    (if (< _targetarmlength _springarmlength)
      (bind (_direction _armlength _armpitch) (`Timeline|MoveToTopDown` :!label _label_5)
        (:`Update`
          (set `SpringArmComponent.TargetArmLength` _armlength _springarm_2)
          (`SceneComponent.K2_SetRelativeRotation` _springarm_2 (`KismetMathLibrary.MakeRotator` _relativerotation_roll_2 _armpitch _relativerotation_yaw) false false)))
      (else
        (goto _label_5 :!via `Reverse`)))))

(fn `Add EXP`
  (params (EXP :type Integer))
  (returns (Level :type Integer))
  (bind _output_get (set `self.EXP` (+ EXP (`self.EXP`))))
  (if (>= _output_get (`self.EXP_Needed`))
    (`/Engine/EditorBlueprintResources/StandardMacros.IncrementInt` (`self.Level`)
      (:`  `
        (set `self.EXP` (- (`self.EXP`) (`self.EXP_Needed`)))
        (set `self.EXP_Needed` (`KismetMathLibrary.Clamp` (`KismetMathLibrary.FTrunc` (* (`self.EXP_Needed`) 1.2)) 0 100))
        (return (`self.Level`))))))

(fn `UpdateHealth`
  (params (health :type "Float (double-precision)"))
  (`/Engine/EditorBlueprintResources/StandardMacros.CompareFloat` health 100.0
    (:`==`
      _)
    (:`<`
      _))
  (bind _output_get (set `self.health` health))
  (bind _asbp_hud (cast `/Game/Blueprints/BP_HUD` (`PlayerController.GetHUD` (`GameplayStatics.GetPlayerController` 0))))
  (`/Game/Blueprints/BP_HUD.UpdateHealth` _asbp_hud (/ _output_get 100.0)))

(fn `UpdateMana`
  (params (mana :type "Float (double-precision)"))
  (`/Engine/EditorBlueprintResources/StandardMacros.CompareFloat` mana 150.0
    (:`==`
      _)
    (:`<`
      _))
  (bind _output_get (set `self.mana` mana))
  (bind _asbp_hud (cast `/Game/Blueprints/BP_HUD` (`PlayerController.GetHUD` (`GameplayStatics.GetPlayerController` 0))))
  (`/Game/Blueprints/BP_HUD.UpdateMana` _asbp_hud (/ _output_get 150.0)))

(fn `UpdateStamina`
  (params (stamina :type "Float (double-precision)"))
  (`/Engine/EditorBlueprintResources/StandardMacros.CompareFloat` stamina 100.0
    (:`==`
      _)
    (:`<`
      _))
  (bind _output_get (set `self.stamina` stamina))
  (bind _asbp_hud (cast `/Game/Blueprints/BP_HUD` (`PlayerController.GetHUD` (`GameplayStatics.GetPlayerController` 0))))
  (`/Game/Blueprints/BP_HUD.UpdateStamina` _asbp_hud (/ _output_get 100.0)))

(fn `UserConstructionScript`)